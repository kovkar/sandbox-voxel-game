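; Voxel terrain chunk actor that builds its block data and visible surface in the construction script, using settings from a World reference.
; LoadChunk samples 2D noise at chunk-offset coordinates for each column's height, then fills a flattened 3D voxel array with grass, snow above a threshold, or the default value above ground.
; Only each column's top voxel is rendered, as an instance in the grass or snow instanced static mesh.
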(fn ConstructionScript
  (bind _world (Variables|Default|GetWorld))
  (bind _chunksize (Variables|/Game/Blueprints/AWorld.AWorld_C|GetChunkSize _world))
  (Utilities|Array|Resize (Variables|Chunk|GetVoxels) (* _chunksize _chunksize (Variables|/Game/Blueprints/AWorld.AWorld_C|GetMaxHeight _world)))
  (CallFunction|LoadChunk))

(fn GetTerrainHeight
  (params (VoxelX :type Integer) (VoxelY :type Integer))
  (return (Math|Float|Floor (Math|Float|MapRangeUnclamped (Class|FastNoiseWrapper|GetNoise2D (Variables|/Game/Blueprints/AWorld.AWorld_C|GetNoise (Variables|Default|GetWorld)) (Math|Conversions|ToFloat(Integer) (+ VoxelX (* (Variables|Chunk|GetChunkPosX) (Variables|/Game/Blueprints/AWorld.AWorld_C|GetChunkSize (Variables|Default|GetWorld))))) (Math|Conversions|ToFloat(Integer) (+ VoxelY (* (Variables|Chunk|GetChunkPosY) (Variables|/Game/Blueprints/AWorld.AWorld_C|GetChunkSize (Variables|Default|GetWorld)))))) -1.0 1.0 0.0 (Math|Conversions|ToFloat(Integer) (Variables|/Game/Blueprints/AWorld.AWorld_C|GetMaxHeight (Variables|Default|GetWorld)))))))

(fn LoadChunk
  (bind _world (Variables|Default|GetWorld))
  (bind _chunksize (Variables|/Game/Blueprints/AWorld.AWorld_C|GetChunkSize _world))
  (bind _returnvalue (- _chunksize 1))
  (for _index (range 0 _returnvalue) ; X
    (LocalVariables|SetVoxelX _index)
    (for _index_2 (range 0 _returnvalue) ; Y
      (LocalVariables|SetVoxelY _index_2)
      (bind _voxelheight (CallFunction|GetTerrainHeight (LocalVariables|GetVoxelX) (LocalVariables|GetVoxelY)))
      (LocalVariables|SetTerrainHeight _voxelheight)
      (for _index_3 (range 0 (- (Variables|/Game/Blueprints/AWorld.AWorld_C|GetMaxHeight (Variables|Default|GetWorld)) 1)) ; Z
        (bind _output_get (LocalVariables|SetVoxelZ _index_3))
        (if (> _output_get (LocalVariables|GetTerrainHeight))
          (CallFunction|SetVoxel (LocalVariables|GetVoxelX) (LocalVariables|GetVoxelY) (LocalVariables|GetVoxelZ) "NewEnumerator0")
          (elif (>= (LocalVariables|GetVoxelZ) (Variables|/Game/Blueprints/AWorld.AWorld_C|GetSnowThresh (Variables|Default|GetWorld)))
            (CallFunction|SetVoxel (LocalVariables|GetVoxelX) (LocalVariables|GetVoxelY) (LocalVariables|GetVoxelZ) "NewEnumerator2")
            (else
              (CallFunction|SetVoxel (LocalVariables|GetVoxelX) (LocalVariables|GetVoxelY) (LocalVariables|GetVoxelZ) "NewEnumerator1")))))
      (CallFunction|InstantiateVoxel (LocalVariables|GetVoxelX) (LocalVariables|GetVoxelY) (LocalVariables|GetTerrainHeight)))))

(fn SetVoxel
  (params (VoxelX :type Integer) (VoxelY :type Integer) (VoxelZ :type Integer) (Value :type EVoxelType%20Enum :default "NewEnumerator0"))
  (bind _flatindex (CallFunction|FlattenIndex VoxelX VoxelY VoxelZ))
  (Utilities|Array|SetArrayElem (Variables|Chunk|GetVoxels) _flatindex Value))

(fn FlattenIndex
  (params (x :type Integer) (y :type Integer) (z :type Integer))
  (bind _world (Variables|Default|GetWorld))
  (bind _maxheight (Variables|/Game/Blueprints/AWorld.AWorld_C|GetMaxHeight _world))
  (return (+ z (* x (Variables|/Game/Blueprints/AWorld.AWorld_C|GetChunkSize (Variables|Default|GetWorld)) _maxheight) (* _maxheight y))))

(fn GetVoxel
  (params (x :type Integer) (y :type Integer) (z :type Integer))
  (bind _flatindex (CallFunction|FlattenIndex x y z))
  (return (Utilities|Array|Get(acopy) (Variables|Chunk|GetVoxels) _flatindex)))

(fn InstantiateVoxel
  (params (x :type Integer) (y :type Integer) (z :type Integer))
  (bind _returnvalue (Math|Conversions|ToFloat(Integer) x))
  (bind _returnvalue_2 (Math|Conversions|ToFloat(Integer) y))
  (bind _returnvalue_3 (Math|Conversions|ToFloat(Integer) z))
  (bind _world (Variables|Default|GetWorld))
  (bind _returnvalue_4 (Math|Vector|MakeVector _returnvalue _returnvalue_2 _returnvalue_3))
  (bind _voxeloffset (Variables|/Game/Blueprints/AWorld.AWorld_C|GetVoxelOffset _world))
  (bind _returnvalue_5 (* _returnvalue_4 _voxeloffset))
  (bind _returnvalue_6 (Math|Transform|MakeTransform _returnvalue_5))
  (bind _voxel (CallFunction|GetVoxel x y z))
  (switch Utilities|FlowControl|Switch|SwitchonEVoxelType _voxel
    (:NewEnumerator1
      (Components|InstancedStaticMesh|AddInstance (Variables|Default|GetISM_Grass) _returnvalue_6 false))
    (:NewEnumerator2
      (Components|InstancedStaticMesh|AddInstance (Variables|Default|GetISM_Snow) _returnvalue_6 false))))