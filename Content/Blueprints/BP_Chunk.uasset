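; Voxel terrain chunk that builds a Perlin-noise heightmap surface from instanced grass and snow blocks.
; The construction script creates a FastNoiseWrapper, which GenerateTerrain uses after clearing both instanced meshes and looping over a ChunkSize grid.
; Each column gets one block at a floored noise height sampled from chunk-local indices, scaled by VoxelSize.
; Blocks at or above SnowThresh use the snow mesh, the rest grass.
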(event Custom|GenerateTerrain
  (bind _chunksize (Variables|Default|GetChunkSize))
  (CallFunction|ClearTerrain)
  (for _index (range 1 _chunksize)
    (for _index_2 (range 1 _chunksize)
      (CallFunction|InstantiateTerrainBlock (Math|Vector|MakeVector (Math|Conversions|ToFloat(Integer) _index_2) (Math|Conversions|ToFloat(Integer) _index) 0.0)))))

(event Custom|ClearTerrain
  (Components|InstancedStaticMesh|ClearInstances (Variables|Default|GetISM_Grass))
  (Components|InstancedStaticMesh|ClearInstances (Variables|Default|GetISM_Snow)))

(fn ConstructionScript
  (bind _returnvalue (Game|ConstructObjectfromClass "/Script/FastNoiseGenerator.FastNoiseWrapper"))
  (bind _output_get (Variables|Default|SetNoise _returnvalue))
  (Class|FastNoiseWrapper|SetupFastNoise _output_get "Perlin" 1337 0.05 "Quintic" "FBM" 3 2.0 0.5 0.45 "Euclidean" "CellValue"))

(fn InstantiateTerrainBlock
  (params (VoxelPos :type Vector))
  (bind _chunkheight (Variables|Default|GetChunkHeight))
  (bind _voxelsize (Variables|Default|GetVoxelSize))
  (bind _noise (Variables|Default|GetNoise))
  (bind _returnvalue (Math|Conversions|ToFloat(Integer) _chunkheight))
  (bind _returnvalue_2 (Class|FastNoiseWrapper|GetNoise2D _noise (.x VoxelPos) (.y VoxelPos)))
  (bind _returnvalue_3 (Math|Float|MapRangeUnclamped _returnvalue_2 -1.0 1.0 0.0 _returnvalue))
  (bind _returnvalue_4 (Math|Float|Floor _returnvalue_3))
  (bind _returnvalue_5 (Math|Conversions|ToFloat(Integer) _returnvalue_4))
  (bind _returnvalue_6 (Math|Vector|MakeVector (.x VoxelPos) (.y VoxelPos) _returnvalue_5))
  (bind _returnvalue_7 (* _returnvalue_6 _voxelsize))
  (if (>= _returnvalue_4 (Variables|Default|GetSnowThresh))
    (Components|InstancedStaticMesh|AddInstance (Variables|Default|GetISM_Snow) (Math|Transform|MakeTransform _returnvalue_7 "0, 0, 0" "1.000000,1.000000,1.000000") false)
    (else
      (Components|InstancedStaticMesh|AddInstance (Variables|Default|GetISM_Grass) (Math|Transform|MakeTransform _returnvalue_7 "0, 0, 0" "1.000000,1.000000,1.000000") false))))