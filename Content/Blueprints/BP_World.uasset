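; BP_World is the root actor of what appears to be a chunked voxel world, owning the shared noise generator and starting chunk creation.
; On BeginPlay it builds a FastNoiseWrapper set to Perlin noise from its Seed and NoiseFreq variables.
; It then spawns a single BP_Chunk at the origin, passing the chunk position and a reference to itself.
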(event EventBeginPlay
  ;[1 1 1] Setup noise generator
  (bind _returnvalue (Game|ConstructObjectfromClass "/Script/FastNoiseGenerator.FastNoiseWrapper"))
  (bind _output_get (Variables|Default|SetNoise _returnvalue))
  (Class|FastNoiseWrapper|SetupFastNoise _output_get "Perlin" (Variables|TerrainSettings|GetSeed) (Variables|TerrainSettings|GetNoiseFreq) "Quintic" "FBM" 3 2.0 0.5 0.45 "Euclidean" "CellValue")
  ;[1 1 1] Spawn initial chunk
  (Game|SpawnActorfromClass "/Game/Blueprints/BP_Chunk.BP_Chunk_C" (Math|Transform|MakeTransform "0, 0, 0") "Undefined" "MultiplyWithRoot" 0 (Math|Vector|MakeVector 0.0 0.0 0.0) self 0))

(fn ConstructionScript)